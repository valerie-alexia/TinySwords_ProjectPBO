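; Game mode that spawns the player's chosen hero when play begins.
; BeginPlay branches on the HeroSelection value to spawn a Mage, Shooter or Fighter hero Blueprint at one fixed, hardcoded location.
; The first player controller then possesses the new hero, and any other selection value spawns nothing.
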(event EventBeginPlay
  (if (== (Variables|Default|GetHeroSelection) 0)
    (bind _returnvalue (Game|SpawnActorfromClass "/Game/CHARACTERS/Hero/Child_Hero/BP_Hero_Mage.BP_Hero_Mage_C" (Math|Transform|MakeTransform "330.000000,410.000000,19.494362" "0, 0, 0" "1.000000,1.000000,1.000000") "Undefined" "MultiplyWithRoot" 0 0))
    (Pawn|Possess (Game|GetPlayerController 0) _returnvalue)
    (elif (== (Variables|Default|GetHeroSelection) 1)
      (bind _returnvalue_2 (Game|SpawnActorfromClass "/Game/CHARACTERS/Hero/Child_Hero/BP_Hero_Shooter.BP_Hero_Shooter_C" (Math|Transform|MakeTransform "330.000000,410.000000,19.494362" "0, 0, 0" "1.000000,1.000000,1.000000") "Undefined" "MultiplyWithRoot" 0 0))
      (Pawn|Possess (Game|GetPlayerController 0) _returnvalue_2)
      (elif (== (Variables|Default|GetHeroSelection) 2)
        (bind _returnvalue_3 (Game|SpawnActorfromClass "/Game/CHARACTERS/Hero/Child_Hero/BP_Hero_Fighter.BP_Hero_Fighter_C" (Math|Transform|MakeTransform "330.000000,410.000000,19.494362" "0, 0, 0" "1.000000,1.000000,1.000000") "Undefined" "MultiplyWithRoot" 0 0))
        (Pawn|Possess (Game|GetPlayerController 0) _returnvalue_3)))))

(event EventTick
  (params (DeltaSeconds :type Float%20%28single-precision%29)))

(fn ConstructionScript)