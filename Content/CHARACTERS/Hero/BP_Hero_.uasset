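; BP_Hero is the player hero: a sprite-based character moved along the world X and Y axes with Enhanced Input.
; BeginPlay shows the mouse cursor and, if the input subsystem is valid, adds the movement mapping context and initializes health.
; IA_Movement applies movement input with Y inverted, flips the sprite through its X scale, and stores the input as a Direction vector.
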(event Input|EnhancedActionEvents|EnhancedInputActionIA_Movement
  (params (ActionValue :type Vector%202D%20Structure) (ElapsedSeconds :type Float%20%28double-precision%29) (TriggeredSeconds :type Float%20%28double-precision%29) (InputAction :type Input%20Action%20Object%20Reference :default "/Game/CHARACTERS/Hero/IA_Movement.IA_Movement"))
  ;[1 1 1] MOVEMENT
  (Utilities|FlowControl|Sequence
    (:then_0
      (Pawn|Input|AddMovementInput "1.000000,0.000000,0.000000" (.x ActionValue) false)
      (if (!= (.x ActionValue) 0.0)
        (Transformation|SetWorldScale3D (Variables|Default|GetSprite) (Math|Vector|MakeVector (.x ActionValue) 1.0 1.0))))
    (:then_1
      (Pawn|Input|AddMovementInput "0.000000,-1.000000,0.000000" (.y ActionValue) false))
    (:then_2
      (Variables|Default|SetDirection (Math|Vector|MakeVector (.x ActionValue) (* (.y ActionValue) -1.0) 0.0)))))

(event EventBeginPlay
  (bind _returnvalue (Game|GetPlayerController 0))
  (bind _returnvalue_2 (PlayerController|LocalPlayerSubsystems|GetEnhancedInputLocalPlayerSubsystem _returnvalue))
  ;[1 1 1] PLAY CONTROLLER
  (Variables|/Script/Engine.PlayerController|SetbShowMouseCursor _returnvalue true)
  (Utilities|IsValid _returnvalue_2
    (:Is%20Valid
      (Input|AddMappingContext _returnvalue_2 "/Game/CHARACTERS/Hero/IMC_MovementMapping.IMC_MovementMapping" 0 "(bIgnoreAllPressedKeysUntilRelease=True,bForceImmediately=False,bNotifyUserSettings=False)")
      (Variables|Default|SetMax%20Health 1e+02)
      (Variables|Default|SetHealth 1e+02))))

(event Collision|EventActorBeginOverlap
  (params (OtherActor :type Actor%20Object%20Reference)))

(event EventTick
  (params (DeltaSeconds :type Float%20%28single-precision%29)))

(fn ConstructionScript)