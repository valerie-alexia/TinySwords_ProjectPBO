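; BP_Hero_Shooter is a hero shooting Blueprint that spawns projectiles aimed at the mouse cursor while the IA_MageShoot input is held.
; The input opens and closes a Gate on Tick, and a short Delay behind it throttles the fire rate.
; Each projectile spawns at a small world-X offset from player 0's pawn, rotated toward the Visibility trace hit under the cursor.
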(event Input|EnhancedActionEvents|EnhancedInputActionIA_MageShoot
  (params (ActionValue :type Float%20%28double-precision%29) (ElapsedSeconds :type Float%20%28double-precision%29) (TriggeredSeconds :type Float%20%28double-precision%29) (InputAction :type Input%20Action%20Object%20Reference :default "/Game/CHARACTERS/Hero/IA_MageShoot.IA_MageShoot"))
  (bind _returnvalue (Game|GetPlayerController 0))
  (bind _returnvalue_2 (Pawn|GetControlledPawn _returnvalue))
  (bind _returnvalue_3 (Transformation|GetActorLocation _returnvalue_2))
  ;[1 1 1] shoot start location
  (:Started
    (Utilities|FlowControl|Gate true) ; enters at Open
  )
  (:Completed
    (Utilities|FlowControl|Gate true) ; enters at Close
  ))

(event EventBeginPlay)

(event Collision|EventActorBeginOverlap
  (params (OtherActor :type Actor%20Object%20Reference)))

(event EventTick
  (params (DeltaSeconds :type Float%20%28single-precision%29))
  (bind _returnvalue (Game|GetPlayerController 0))
  (bind _returnvalue_2 (Pawn|GetControlledPawn _returnvalue))
  (bind _returnvalue_3 (Transformation|GetActorLocation _returnvalue_2))
  ;[1 1 1] shoot start location
  (Utilities|FlowControl|Gate true
    (:Exit
      (Utilities|FlowControl|Delay 0.2)
      (Game|SpawnActorfromClass (Variables|Default|GetProjectile) (Math|Transform|MakeTransform (+ _returnvalue_3 "5.000000,0.000000,0.000000") (Math|Rotator|FindLookatRotation _returnvalue_3 (.Location (Collision|BreakHitResult (.HitResult (Game|Player|GetHitResultUnderCursorbyChannel _returnvalue "TraceTypeQuery1" true)))))) "Undefined" "MultiplyWithRoot" 0 0))))

(fn ConstructionScript)