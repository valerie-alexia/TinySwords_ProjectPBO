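; Shooter hero, a child Blueprint that sets its own health, damage and run flipbook on BeginPlay.
; IA_shootHit spawns a projectile aimed from the pawn at the cursor hit, chosen by the GameInstance's WeaponChoosing: infinite-range arrow, a spawn with no class set, or explosive arrow.
; A boolean and Delay form a per-weapon fire cooldown.
; The sprite returns to the idle flipbook when playback finishes.
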(event OnFinishedPlaying(Sprite)
  (Sprite|SetFlipbook (Variables|Default|GetSprite) "/Game/Asset/Tiny_Swords__Update_010_/Factions/Knights/Troops/Archer/Blue/Idle_Shooter.Idle_Shooter")
  (Components|Timeline|SetLooping (Variables|Default|GetSprite) false)
  (if (not (Audio|Components|Audio|IsPlaying (Variables|Default|GetSprite)))
    (Audio|Components|Audio|Play (Variables|Default|GetSprite))))

(event Input|EnhancedActionEvents|EnhancedInputActionIA_shootHit
  (params (ActionValue :type Float%20%28double-precision%29) (ElapsedSeconds :type Float%20%28double-precision%29) (TriggeredSeconds :type Float%20%28double-precision%29) (InputAction :type Input%20Action%20Object%20Reference :default "/Game/CHARACTERS/Hero/InputAction/IA_shootHit.IA_shootHit"))
  (bind _returnvalue (Game|GetPlayerController 0))
  (bind _returnvalue_2 (Pawn|GetControlledPawn _returnvalue))
  (bind _hitresult (Game|Player|GetHitResultUnderCursorbyChannel _returnvalue "TraceTypeQuery1" true))
  (bind _returnvalue_3 (Transformation|GetActorLocation _returnvalue_2))
  (bind _location (Collision|BreakHitResult _hitresult))
  (bind _returnvalue_4 (Math|Rotator|FindLookatRotation _returnvalue_3 _location))
  (bind _returnvalue_5 (+ _returnvalue_3 "5.000000,0.000000,0.000000"))
  (bind _returnvalue_6 (Math|Transform|MakeTransform _returnvalue_5 _returnvalue_4))
  (:Started
    ;[1 0.8941 0.2667] shoot start location
    (bind _asbp_game_instanes (Utilities|Casting|CastToBP_GameInstanes (Game|GetGameInstance)))
    (if (and (Variables|Default|GetFirst?) (== (Variables|/Game/MainMenu/BP_GameInstanes.BP_GameInstanes_C|GetWeaponChoosing _asbp_game_instanes) 0))
      (Game|SpawnActorfromClass "/Game/CHARACTERS/ShooterWeapon/BP_Projectile_Arrow_InfinRange.BP_Projectile_Arrow_InfinRange_C" _returnvalue_6 "Undefined" "MultiplyWithRoot" 0 0)
      (Variables|Default|SetFirst? false)
      (Utilities|FlowControl|Delay 0.6)
      (Variables|Default|SetFirst? true)
      (elif (and (Variables|Default|GetFirst?) (== (Variables|/Game/MainMenu/BP_GameInstanes.BP_GameInstanes_C|GetWeaponChoosing _asbp_game_instanes) 1))
        (Game|SpawnActorfromClass "/Game/CHARACTERS/ShooterWeapon/BP_Projectile_Arrow_RapidFire.BP_Projectile_Arrow_RapidFire_C" _returnvalue_6 "Undefined" "MultiplyWithRoot" 0 0)
        (Variables|Default|SetFirst? false)
        (Utilities|FlowControl|Delay 0.2)
        (Variables|Default|SetFirst? true)
        (elif (and (Variables|Default|GetFirst?) (== (Variables|/Game/MainMenu/BP_GameInstanes.BP_GameInstanes_C|GetWeaponChoosing _asbp_game_instanes) 2))
          (Game|SpawnActorfromClass "/Game/CHARACTERS/ShooterWeapon/BP_Projectile_Arrow_Explosive.BP_Projectile_Arrow_Explosive_C" _returnvalue_6 "Undefined" "MultiplyWithRoot" 0 0)
          (Variables|Default|SetFirst? false)
          (Utilities|FlowControl|Delay 0.6)
          (Variables|Default|SetFirst? true))))))

(event EventBeginPlay
  (|CallParentFunction)
  (Variables|Default|SetAttackDamage 3e+01)
  (bind _output_get (Variables|Default|SetMax%20Health 1e+03))
  (Variables|Default|SetHealth _output_get)
  (Variables|Default|SetRunFlipbook "/Game/Asset/Hero_Asset/Shooter_Asset/Blue/Run_Shooter.Run_Shooter"))

(event Collision|EventActorBeginOverlap
  (params (OtherActor :type Actor%20Object%20Reference)))

(event EventTick
  (params (DeltaSeconds :type Float%20%28single-precision%29)))

(fn ConstructionScript)