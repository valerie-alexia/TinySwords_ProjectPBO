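; Mage child hero Blueprint that sets its own health, attack damage and run flipbook after the parent BeginPlay.
; The shoot input spawns the selected skill projectile near player 0's pawn, rotated toward the cursor trace hit.
; A boolean gate and Delay enforce the attack cooldown.
; The switch input advances a wrapping counter that cycles the skill through basic projectile, fireball and iceball.
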(event Input|EnhancedActionEvents|EnhancedInputActionIA_shootHit
  (params (ActionValue :type Float%20%28double-precision%29) (ElapsedSeconds :type Float%20%28double-precision%29) (TriggeredSeconds :type Float%20%28double-precision%29) (InputAction :type Input%20Action%20Object%20Reference :default "/Game/CHARACTERS/Hero/InputAction/IA_shootHit.IA_shootHit"))
  (bind _returnvalue (Game|GetPlayerController 0))
  (bind _returnvalue_2 (Pawn|GetControlledPawn _returnvalue))
  (bind _returnvalue_3 (Transformation|GetActorLocation _returnvalue_2))
  ;[1 1 1] shoot start location
  (:Started
    (if (Variables|Default|GetFirst?)
      (Game|SpawnActorfromClass (Variables|Default|GetMageSkill) (Math|Transform|MakeTransform (+ _returnvalue_3 "5.000000,0.000000,0.000000") (Math|Rotator|FindLookatRotation _returnvalue_3 (.Location (Collision|BreakHitResult (.HitResult (Game|Player|GetHitResultUnderCursorbyChannel _returnvalue "TraceTypeQuery1" true)))))) "Undefined" "MultiplyWithRoot" 0 0)
      (Variables|Default|SetFirst? false)
      (Utilities|FlowControl|Delay (Variables|Default|GetAttackCD))
      (Variables|Default|SetFirst? true))))

(event Input|EnhancedActionEvents|EnhancedInputActionIA_SwitchSkill
  (params (ActionValue :type Boolean) (ElapsedSeconds :type Float%20%28double-precision%29) (TriggeredSeconds :type Float%20%28double-precision%29) (InputAction :type Input%20Action%20Object%20Reference :default "/Game/CHARACTERS/Hero/InputAction/IA_SwitchSkill.IA_SwitchSkill"))
  ;[1 1 1] Switch Skills
  (:Started
    (Utilities|FlowControl|Sequence
      (:then_0
        (Math|Integer|IncrementInt (Variables|Default|Getcounter)))
      (:then_1
        (if (!= (Variables|Default|Getcounter) 3) :!label _label
          (if (== (Variables|Default|Getcounter) 0)
            (Variables|Default|SetMageSkill "/Game/CHARACTERS/Projectiles/MageSkill/BP_Projectile.BP_Projectile_C")
            (elif (== (Variables|Default|Getcounter) 1)
              (Variables|Default|SetMageSkill "/Game/CHARACTERS/Projectiles/MageSkill/BP_Projectile_FireBall.BP_Projectile_FireBall_C")
              (elif (== (Variables|Default|Getcounter) 2)
                (Variables|Default|SetMageSkill "/Game/CHARACTERS/Projectiles/MageSkill/BP_Projectile_IceBall.BP_Projectile_IceBall_C"))))
          (else
            (Variables|Default|Setcounter 0)
            (goto _label)))))))

(event EventBeginPlay
  ;[1 1 1] Stats
  (|CallParentFunction)
  (Variables|Default|SetAttackDamage 1e+01)
  (bind _output_get (Variables|Default|SetMax%20Health 3e+02))
  (Variables|Default|SetHealth _output_get)
  (Variables|Default|SetRunFlipbook "/Game/Asset/Hero_Asset/Mage_Asset/Mage/Blue/Run_Mage.Run_Mage"))

(event Collision|EventActorBeginOverlap
  (params (OtherActor :type Actor%20Object%20Reference)))

(event EventTick
  (params (DeltaSeconds :type Float%20%28single-precision%29))
  ;[1 1 1] shoot start location
)

(fn ConstructionScript)