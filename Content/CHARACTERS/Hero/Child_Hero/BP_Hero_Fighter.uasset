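; Melee fighter hero Blueprint that sets its own health and damage, then attacks monsters using flipbook animations.
; IA_shootHit Started fires a light attack, while Triggered fires a heavier one after a delay, each setting damage and animation.
; Both call HitCheck, which damages BP_Monster actors overlapping the HitBox at that instant, and unhide the HitBox.
; When a flipbook finishes, the sprite returns to idle, IsAttacking clears and the HitBox hides.
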(event OnFinishedPlaying(Sprite)
  (Sprite|SetFlipbook (Variables|Default|GetSprite) "/Game/Asset/Hero_Asset/Fighter_Asset/Fighter/Blue/Idle_Fighter.Idle_Fighter")
  (CallFunction|RestartAnim)
  (Variables|Default|SetIs%20Attacking false)
  (Development|SetHiddeninGame (Variables|Default|GetHitBox) true false))

(event Input|EnhancedActionEvents|EnhancedInputActionIA_shootHit
  (params (ActionValue :type Float%20%28double-precision%29) (ElapsedSeconds :type Float%20%28double-precision%29) (TriggeredSeconds :type Float%20%28double-precision%29) (InputAction :type Input%20Action%20Object%20Reference :default "/Game/CHARACTERS/Hero/InputAction/IA_shootHit.IA_shootHit"))
  (:Triggered
    ;[1 1 1] Heavy Attack
    (Utilities|FlowControl|Delay 3.0)
    (Variables|Default|SetAttackDamage 2e+01)
    (Sprite|SetFlipbook (Variables|Default|GetSprite) "/Game/Asset/Hero_Asset/Fighter_Asset/Fighter/Blue/FullAttack_Fighter.FullAttack_Fighter")
    (Components|Timeline|SetLooping (Variables|Default|GetSprite) false)
    (Variables|Default|SetIs%20Attacking true)
    (CallFunction|HitCheck)
    (Development|SetHiddeninGame (Variables|Default|GetHitBox) false false))
  (:Started
    ;[1 1 1] Light Attack
    (Variables|Default|SetAttackDamage 1e+01)
    (Sprite|SetFlipbook (Variables|Default|GetSprite) "/Game/Asset/Hero_Asset/Fighter_Asset/Fighter/Blue/Attack_Fighter.Attack_Fighter")
    (Components|Timeline|SetLooping (Variables|Default|GetSprite) false)
    (Variables|Default|SetIs%20Attacking true)
    (CallFunction|HitCheck)
    (Development|SetHiddeninGame (Variables|Default|GetHitBox) false false)))

(event EventBeginPlay
  (|CallParentFunction)
  (Variables|Default|SetAttackDamage 8e+01)
  (Variables|Default|SetMax%20Health 2e+02)
  (Variables|Default|SetHealth 2e+02))

(event EventTick
  (params (DeltaSeconds :type Float%20%28single-precision%29)))

(event Collision|EventActorBeginOverlap
  (params (OtherActor :type Actor%20Object%20Reference)))

(fn ConstructionScript)

(fn RestartAnim
  (Components|Timeline|SetLooping (Variables|Default|GetSprite) false)
  (if (not (Audio|Components|Audio|IsPlaying (Variables|Default|GetSprite)))
    (Audio|Components|Audio|Play (Variables|Default|GetSprite))))

(fn HitCheck
  (bind _attackdamage (Variables|Default|GetAttackDamage))
  (for _array_element (Collision|GetOverlappingActors (Variables|Default|GetHitBox) "/Game/CHARACTERS/Monster/BP_Monster.BP_Monster_C" :!class /Script/Engine.PrimitiveComponent)
    (if (!= _array_element self)
      (Game|Damage|ApplyDamage _array_element _attackdamage 0 self "/Script/Engine.DamageType")
      (Development|PrintString (Utilities|String|ToString(Float) _attackdamage)))))

(fn SetAnimState
  (Components|Timeline|SetLooping (Variables|Default|GetSprite) false))