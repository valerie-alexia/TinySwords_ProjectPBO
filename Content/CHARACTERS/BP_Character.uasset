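; BP_Character is a character Blueprint with a simple health and death system.
; On any damage, it subtracts the amount from Health, clamped between zero and MaxHealth, unless it is already dead.
; When Health reaches zero, it sets IsDead and destroys the actor immediately.
; BeginPlay only prints a debug greeting, and the overlap, tick and construction script are empty.
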(event EventBeginPlay
  (Development|PrintString "Hello"))

(event Collision|EventActorBeginOverlap
  (params (OtherActor :type Actor%20Object%20Reference)))

(event EventTick
  (params (DeltaSeconds :type Float%20%28single-precision%29)))

(event Game|Damage|EventAnyDamage
  (params (Damage :type Float%20%28single-precision%29) (DamageType :type Damage%20Type%20Object%20Reference) (InstigatedBy :type Controller%20Object%20Reference) (DamageCauser :type Actor%20Object%20Reference))
  ;[1 1 1] DAMAGE SYSTEM
  (if (not (Variables|Default|Getis%20Dead?))
    (bind _output_get (Variables|Default|SetHealth (Math|Float|Clamp(Float) (- (Variables|Default|GetHealth) Damage) 0.0 (Variables|Default|GetMax%20Health))))
    (if (<= _output_get 0.0)
      (Variables|Default|Setis%20Dead? true)
      (Actor|DestroyActor))))

(fn ConstructionScript)