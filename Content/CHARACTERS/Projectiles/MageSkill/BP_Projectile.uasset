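; Mage skill projectile Blueprint that damages non-hero actors it touches and expires after one second.
; On spawn it sets the attack cooldown on the BP_Hero_Mage found in the world.
; Capsule overlaps ignore heroes; any other actor takes damage and the projectile destroys itself, also calling ReturnNormalAfterHurt on monsters.
; The damage causer comes from the failed hero cast, so it is null.
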(event OnComponentBeginOverlap(Capsule)
  (params (OverlappedComponent :type Primitive%20Component%20Object%20Reference) (OtherActor :type Actor%20Object%20Reference) (OtherComp :type Primitive%20Component%20Object%20Reference) (OtherBodyIndex :type Integer) (bFromSweep :type Boolean) (SweepResult :type Hit%20Result%20Structure%20%28by%20ref%29))
  ;[1 1 1] If themself, no harm
  (bind _asbp_hero_ (Utilities|Casting|CastToBP_Hero_ OtherActor)
    (:CastFailed
      (Game|Damage|ApplyDamage OtherActor (Variables|Default|GetDamage) 0 _asbp_hero_ "/Script/Engine.DamageType")
      (Actor|DestroyActor)
      (bind _asbp_monster (Utilities|Casting|CastToBP_Monster OtherActor))
      (Utilities|Casting|CastToBP_Character (Game|GetPlayerCharacter 0))
      (Default|ReturnNormalAfterHurt _asbp_monster))))

(event EventBeginPlay
  (bind _returnvalue (Actor|GetActorOfClass "/Game/CHARACTERS/Hero/Child_Hero/BP_Hero_Mage.BP_Hero_Mage_C"))
  (Actor|SetLifeSpan 1.0)
  (Variables|/Game/CHARACTERS/Hero/Parent_Hero/BP_Hero_.BP_Hero__C|SetAttackCD _returnvalue 0.2))

(event EventTick
  (params (DeltaSeconds :type Float%20%28single-precision%29)))

(fn ConstructionScript)