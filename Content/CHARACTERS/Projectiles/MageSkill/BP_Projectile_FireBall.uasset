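; Fireball projectile for the Mage hero, a child Blueprint that relies on its parent for any behavior beyond stats and hit animation.
; On BeginPlay it sets its damage, then casts player character 0 to BP_Hero_Mage and writes that hero's attack cooldown, so the projectile itself drives the fire rate.
; When the capsule overlaps a BP_Monster, the Fireballs flipbook switches to the hit animation.
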(event OnComponentBeginOverlap(Capsule)
  (params (OverlappedComponent :type Primitive%20Component%20Object%20Reference) (OtherActor :type Actor%20Object%20Reference) (OtherComp :type Primitive%20Component%20Object%20Reference) (OtherBodyIndex :type Integer) (bFromSweep :type Boolean) (SweepResult :type Hit%20Result%20Structure%20%28by%20ref%29))
  ;[1 1 1] Change Launch & Hit animation
  (Utilities|Casting|CastToBP_Monster OtherActor)
  (Sprite|SetFlipbook (Variables|Default|GetFireballs) "/Game/Asset/MageSkills_Asset/Fire_Effect_1/FireBallHit.FireBallHit"))

(event EventBeginPlay
  ;[1 1 1] Stats
  (|CallParentFunction)
  (Variables|Default|SetDamage 35.0)
  (bind _asbp_hero_mage (Utilities|Casting|CastToBP_Hero_Mage (Game|GetPlayerCharacter 0)))
  (Variables|/Game/CHARACTERS/Hero/Parent_Hero/BP_Hero_.BP_Hero__C|SetAttackCD _asbp_hero_mage 0.5))

(event Collision|EventActorBeginOverlap
  (params (OtherActor :type Actor%20Object%20Reference))
  (|CallParentFunction OtherActor) ; This node is disabled and will not be called.\nDrag off pins to build functionality.
)

(event EventTick
  (params (DeltaSeconds :type Float%20%28single-precision%29))
  (|CallParentFunction DeltaSeconds) ; This node is disabled and will not be called.\nDrag off pins to build functionality.
)

(fn ConstructionScript
  (|CallParentFunction))