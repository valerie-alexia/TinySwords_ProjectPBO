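; Ice ball projectile for the Mage hero that chills and slows the monsters it hits.
; On BeginPlay it sets its damage and the attack cooldown of the player's Mage.
; On capsule overlap with a BP_Monster it switches to the hit flipbook, tints the monster's sprite blue and lowers its walk speed.
; It then calls the monster's ReturnNormal, leaving recovery to the monster.
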(event OnComponentBeginOverlap(Capsule)
  (params (OverlappedComponent :type Primitive%20Component%20Object%20Reference) (OtherActor :type Actor%20Object%20Reference) (OtherComp :type Primitive%20Component%20Object%20Reference) (OtherBodyIndex :type Integer) (bFromSweep :type Boolean) (SweepResult :type Hit%20Result%20Structure%20%28by%20ref%29))
  ;[1 1 1] Change Launch & Hit animation
  (bind _asbp_monster (Utilities|Casting|CastToBP_Monster OtherActor))
  (Sprite|SetFlipbook (Variables|Default|GetIceBalls) "/Game/Asset/MageSkills_Asset/Ice_Effect_01/Ice_Effect_01/Ice_VFX_1/IceHit.IceHit")
  ;[1 1 1] Slowdown Ice
  (Sprite|SetSpriteColor (Variables|/Script/Paper2D.PaperCharacter|GetSprite _asbp_monster) "(R=0.000000,G=0.371483,B=1.000000,A=1.000000)")
  (Variables|/Script/Engine.CharacterMovementComponent|SetMaxWalkSpeed (Variables|/Script/Engine.Character|GetCharacterMovement _asbp_monster) 3e+02)
  (Default|ReturnNormal _asbp_monster))

(event EventBeginPlay
  (|CallParentFunction)
  (Variables|Default|SetDamage 5.0)
  (bind _asbp_hero_mage (Utilities|Casting|CastToBP_Hero_Mage (Game|GetPlayerCharacter 0)))
  (Variables|/Game/CHARACTERS/Hero/Parent_Hero/BP_Hero_.BP_Hero__C|SetAttackCD _asbp_hero_mage 1.2))

(event Collision|EventActorBeginOverlap
  (params (OtherActor :type Actor%20Object%20Reference))
  (|CallParentFunction OtherActor) ; This node is disabled and will not be called.\nDrag off pins to build functionality.
)

(event EventTick
  (params (DeltaSeconds :type Float%20%28single-precision%29))
  (|CallParentFunction DeltaSeconds) ; This node is disabled and will not be called.\nDrag off pins to build functionality.
)

(fn ConstructionScript
  (|CallParentFunction))