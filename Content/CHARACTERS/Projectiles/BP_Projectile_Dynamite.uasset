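; Dynamite projectile, a child Blueprint apparently fired by monsters to damage heroes, that expires one second after spawning.
; Capsule overlaps ignore monsters and react only to actors tagged Hero that cast to BP_Hero_.
; A hit applies damage from OwnerParent's AttackDamage, then, if the player character is a BP_Character, calls the hero's ReturnNormalAfterHurt and destroys the projectile.
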(event OnComponentBeginOverlap(Capsule)
  (params (OverlappedComponent :type Primitive%20Component%20Object%20Reference) (OtherActor :type Actor%20Object%20Reference) (OtherComp :type Primitive%20Component%20Object%20Reference) (OtherBodyIndex :type Integer) (bFromSweep :type Boolean) (SweepResult :type Hit%20Result%20Structure%20%28by%20ref%29))
  ;[1 1 1] If themself, no harm
  (bind _asbp_monster (Utilities|Casting|CastToBP_Monster OtherActor)
    (:CastFailed
      (if (Actor|ActorHasTag OtherActor "Hero")
        (bind _asbp_hero_ (Utilities|Casting|CastToBP_Hero_ OtherActor))
        (Game|Damage|ApplyDamage OtherActor (Variables|/Game/CHARACTERS/BP_Character.BP_Character_C|GetAttackDamage (Variables|Default|GetOwnerParent)) 0 _asbp_monster "/Script/Engine.DamageType")
        (Utilities|Casting|CastToBP_Character (Game|GetPlayerCharacter 0))
        (Default|ReturnNormalAfterHurt _asbp_hero_)
        (Actor|DestroyActor)))))

(event EventBeginPlay
  (|CallParentFunction)
  (Actor|GetActorOfClass "/Game/CHARACTERS/Monster/BP_Monster_Dynamite.BP_Monster_Dynamite_C")
  (Actor|SetLifeSpan 1.0))

(event Collision|EventActorBeginOverlap
  (params (OtherActor :type Actor%20Object%20Reference)))

(event EventTick
  (params (DeltaSeconds :type Float%20%28single-precision%29))
  (|CallParentFunction DeltaSeconds) ; This node is disabled and will not be called.\nDrag off pins to build functionality.
)

(fn ConstructionScript
  (|CallParentFunction))