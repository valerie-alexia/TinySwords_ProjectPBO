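; BP_Projectile_Arrow_Explosive is an explosive arrow projectile for the shooter hero.
; On spawn it limits its own lifespan, sets its damage and overrides the player BP_Hero_Shooter's attack cooldown.
; When its capsule overlaps a BP_Monster, it spawns BP_Explosion at its horizontal position with a fixed height, then destroys itself after a brief delay.
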(event OnComponentBeginOverlap(Capsule)
  (params (OverlappedComponent :type Primitive%20Component%20Object%20Reference) (OtherActor :type Actor%20Object%20Reference) (OtherComp :type Primitive%20Component%20Object%20Reference) (OtherBodyIndex :type Integer) (bFromSweep :type Boolean) (SweepResult :type Hit%20Result%20Structure%20%28by%20ref%29))
  (bind _self self)
  (bind _returnvalue (Transformation|GetActorLocation _self))
  ;[1 1 1] When hit monster
  (Utilities|Casting|CastToBP_Monster OtherActor)
  (Game|SpawnActorfromClass "/Game/CHARACTERS/ShooterWeapon/BP_Explosion.BP_Explosion_C" (Math|Transform|MakeTransform (Math|Vector|MakeVector (.x _returnvalue) (.y _returnvalue) 1e+01) "0, 0, 0" "1.000000,1.000000,1.000000") "Undefined" "MultiplyWithRoot" 0 0)
  (Utilities|FlowControl|Delay 0.1)
  (Actor|DestroyActor))

(event EventBeginPlay
  ;[1 1 1] Arrow default
  (|CallParentFunction)
  (Actor|SetLifeSpan 1.7)
  (bind _asbp_hero_shooter (Utilities|Casting|CastToBP_Hero_Shooter (Game|GetPlayerCharacter 0)))
  (Variables|/Game/CHARACTERS/Hero/Child_Hero/BP_Hero_Shooter.BP_Hero_Shooter_C|SetAttackCD _asbp_hero_shooter 1.0)
  (Variables|Default|SetDamage 5e+01))

(event Collision|EventActorBeginOverlap
  (params (OtherActor :type Actor%20Object%20Reference))
  (|CallParentFunction 0))

(fn ConstructionScript
  (|CallParentFunction))