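; Arrow projectile for the shooter hero's weapon, named as the infinite-range variant and tagged as the default arrow.
; On BeginPlay it runs the parent logic, sets a lifespan that caps its flight time, then sets its damage and overwrites the player's BP_Hero_Shooter attack cooldown.
; The damage assignment follows the hero cast, so it only runs if that cast succeeds.
; Movement and hit handling are left to the parent class.
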(event EventBeginPlay
  ;[1 1 1] Arrow default
  (|CallParentFunction)
  (Actor|SetLifeSpan 1e+01)
  (bind _asbp_hero_shooter (Utilities|Casting|CastToBP_Hero_Shooter (Game|GetPlayerCharacter 0)))
  (Variables|/Game/CHARACTERS/Hero/Parent_Hero/BP_Hero_.BP_Hero__C|SetAttackCD _asbp_hero_shooter 0.7)
  (Variables|Default|SetDamage 1e+01))

(event Collision|EventActorBeginOverlap
  (params (OtherActor :type Actor%20Object%20Reference))
  (|CallParentFunction OtherActor) ; This node is disabled and will not be called.\nDrag off pins to build functionality.
)

(event EventTick
  (params (DeltaSeconds :type Float%20%28single-precision%29))
  (|CallParentFunction DeltaSeconds) ; This node is disabled and will not be called.\nDrag off pins to build functionality.
)

(fn ConstructionScript
  (|CallParentFunction))