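; Wave spawner actor that fills the level with BP_Monster_Archer enemies and announces the end of round 1.
; On BeginPlay it gathers all BP_SpawnMonsterPosition actors, then spawns an archer at a random one each second while CountEnemy stays within MaxEnemy.
; Tick, slowed to a five-second interval, compares BP_Hero_'s CountDeath with MaxEnemy and prints the round-completed message when they match.
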(event EventBeginPlay
  (bind _outactors (Actor|GetAllActorsOfClass "/Game/CHARACTERS/Monster/BP_SpawnMonsterPosition.BP_SpawnMonsterPosition_C"))
  (Variables|Default|SetPosition _outactors)
  (Actor|Tick|SetActorTickInterval 5.0)
  (Game|SpawnActorfromClass "/Game/CHARACTERS/Monster/BP_Monster_Archer.BP_Monster_Archer_C" (Math|Transform|MakeTransform (Transformation|GetActorLocation (.OutItem (Utilities|Array|Random (Variables|Default|GetPosition)))) "0, 0, 0" "1.000000,1.000000,1.000000") "Undefined" "MultiplyWithRoot" 0 0 :!label _label)
  (bind _result (Math|Integer|IncrementInt (Variables|Default|GetCountEnemy))
    (:%20%20
      (Variables|Default|SetCountEnemy _result)
      (Utilities|FlowControl|Delay 1.0)
      (if (<= (Variables|Default|GetCountEnemy) (Variables|Default|GetMax%20Enemy))
        (goto _label)))))

(event Collision|EventActorBeginOverlap
  (params (OtherActor :type Actor%20Object%20Reference)))

(event EventTick
  (params (DeltaSeconds :type Float%20%28single-precision%29))
  (bind _returnvalue (Actor|GetActorOfClass "/Game/CHARACTERS/Hero/Parent_Hero/BP_Hero_.BP_Hero__C"))
  (if (== (Variables|/Game/CHARACTERS/Hero/Parent_Hero/BP_Hero_.BP_Hero__C|GetCount%20Death _returnvalue) (Variables|Default|GetMax%20Enemy))
    (Development|PrintString "ROUND 1 COMPLETED" true true "(R=1.000000,G=0.000000,B=0.991697,A=1.000000)" 5.0)))

(fn ConstructionScript)