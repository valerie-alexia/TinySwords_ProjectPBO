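; BP_Monster_Dynamite is a monster that throws homing dynamite projectiles at the player hero.
; BeginPlay sets the trigger radius and starts a looping timer that spawns BP_Projectile_Dynamite while InThrowRadius is true, homing it on the hero's root component.
; RadiusThrowing's begin overlap sets that flag for a hero and clears it for any other actor.
; No end-overlap handler exists, so leaving the radius does not stop throwing.
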(event OnComponentBeginOverlap(radiusThrowing)
  (params (OverlappedComponent :type Primitive%20Component%20Object%20Reference) (OtherActor :type Actor%20Object%20Reference) (OtherComp :type Primitive%20Component%20Object%20Reference) (OtherBodyIndex :type Integer) (bFromSweep :type Boolean) (SweepResult :type Hit%20Result%20Structure%20%28by%20ref%29))
  (Utilities|Casting|CastToBP_Hero_ OtherActor
    (:then
      (Variables|Default|SetinThrowRadius? true))
    (:CastFailed
      (Variables|Default|SetinThrowRadius? false))))

(event Custom|ThrowDynamite
  (if (Variables|Default|GetinThrowRadius?)
    (bind _returnvalue (Game|SpawnActorfromClass "/Game/CHARACTERS/Projectiles/BP_Projectile_Dynamite.BP_Projectile_Dynamite_C" (Math|Conversions|ToTransform(Vector) (Transformation|GetActorLocation)) "Undefined" "MultiplyWithRoot" 0 self 0))
    (bind _asbp_hero_ (Utilities|Casting|CastToBP_Hero_ (Game|GetPlayerCharacter 0)))
    (Utilities|IsValid (Variables|/Game/CHARACTERS/Projectiles/BP_Projectile_Dynamite.BP_Projectile_Dynamite_C|GetProjectileMovement _returnvalue)
      (:Is%20Valid
        (bind _output_get (Variables|/Script/Engine.ProjectileMovementComponent|SetHomingTargetComponent (Variables|/Game/CHARACTERS/Projectiles/BP_Projectile_Dynamite.BP_Projectile_Dynamite_C|GetProjectileMovement _returnvalue) (Variables|/Script/Engine.Actor|GetRootComponent _asbp_hero_)))))))

(event EventBeginPlay
  (|CallParentFunction)
  (Variables|Default|SetradiusTrigger 2e+02)
  (Utilities|Time|SetTimerbyEvent (delegate Custom|ThrowDynamite) 1.0 true))

(event Collision|EventActorBeginOverlap
  (params (OtherActor :type Actor%20Object%20Reference))
  (|CallParentFunction OtherActor) ; This node is disabled and will not be called.\nDrag off pins to build functionality.
)

(event EventTick
  (params (DeltaSeconds :type Float%20%28single-precision%29))
  (|CallParentFunction DeltaSeconds) ; This node is disabled and will not be called.\nDrag off pins to build functionality.
)

(event EventThrowBomb
  (Variables|Default|SetinThrowRadius? true))

(fn ConstructionScript
  (|CallParentFunction))