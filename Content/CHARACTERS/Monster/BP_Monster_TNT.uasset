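; BP_Monster_TNT is an exploding monster that sets its own health and attack damage on BeginPlay.
; A hero overlapping its capsule starts a looping one-second timer, which ending overlap clears.
; When the timer fires, it damages the hero and increments the player hero's CountDeath without checking for death.
; It then drops its sprite to a low Z, spawns a scaled-up actor and destroys itself after a short delay.
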(event OnComponentBeginOverlap(CapsuleComponent)
  (params (OverlappedComponent :type Primitive%20Component%20Object%20Reference) (OtherActor :type Actor%20Object%20Reference) (OtherComp :type Primitive%20Component%20Object%20Reference) (OtherBodyIndex :type Integer) (bFromSweep :type Boolean) (SweepResult :type Hit%20Result%20Structure%20%28by%20ref%29))
  ;[1 0.3094 0.3094] Explode when overlap
  (bind _asbp_hero_ (Utilities|Casting|CastToBP_Hero_ OtherActor))
  (Development|PrintString "overlap")
  (bind _returnvalue (Utilities|Time|SetTimerbyEvent (delegate Custom|delay%20explode) 1.0 true)))

(event OnComponentEndOverlap(CapsuleComponent)
  (params (OverlappedComponent :type Primitive%20Component%20Object%20Reference) (OtherActor :type Actor%20Object%20Reference) (OtherComp :type Primitive%20Component%20Object%20Reference) (OtherBodyIndex :type Integer))
  ;[1 0.3094 0.3094] Explode when overlap
  (Utilities|Time|ClearandInvalidateTimerbyHandle (stale OnComponentBeginOverlap(CapsuleComponent) _returnvalue)))

(event Custom|delay%20explode
  (bind _self self)
  (bind _returnvalue (Transformation|GetActorLocation _self))
  ;[1 0.3094 0.3094] Explode when overlap
  (Game|Damage|ApplyDamage (stale OnComponentBeginOverlap(CapsuleComponent) _asbp_hero_) (stale EventBeginPlay _output_get) 0 0 "/Script/Engine.DamageType")
  (bind _asbp_hero_ (Utilities|Casting|CastToBP_Hero_ (Game|Player|GetPlayerPawn 0)))
  (Math|Integer|IncrementInt (Variables|/Game/CHARACTERS/Hero/Parent_Hero/BP_Hero_.BP_Hero__C|GetCount%20Death _asbp_hero_)
    (:%20%20
      (Transformation|SetWorldLocation (Variables|Default|GetSprite) (Math|Vector|MakeVector (.x _returnvalue) (.y _returnvalue) -1e+01) false true)
      (Game|SpawnActorfromClass "/Game/CHARACTERS/ShooterWeapon/BP_Explosion.BP_Explosion_C" (Math|Transform|MakeTransform (Math|Vector|MakeVector (.x _returnvalue) (.y _returnvalue) 1e+01) "0, 0, 0" "4.000000,4.000000,4.000000") "Undefined" "MultiplyWithRoot" 0 0)
      (Utilities|FlowControl|Delay 0.5)
      (Actor|DestroyActor))))

(event EventTick
  (params (DeltaSeconds :type Float%20%28single-precision%29))
  (|CallParentFunction DeltaSeconds))

(event EventBeginPlay
  ;[1 0.3094 0.3094] Explode when overlap
  ;;[1 0.9722 0.2874] Stats
  (|CallParentFunction)
  (Variables|Default|SetMax%20Health 5e+01)
  (Variables|Default|SetHealth 5e+01)
  (bind _output_get (Variables|Default|SetAttackDamage 75.0))
  (bind _returnvalue (Actor|GetActorOfClass "/Game/CHARACTERS/Monster/BP_Monster.BP_Monster_C")))

(fn ConstructionScript
  (|CallParentFunction))