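; BP_Monster is a monster Blueprint that chases the player character.
; On BeginPlay it casts player 0's character to BP_Hero, stores it and starts the RunToPlayer event.
; That event runs AI MoveTo toward the hero while Health is nonzero and calls itself again on each success.
; A failed move is not retried, and the graph has no attack or damage logic.
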(event Custom|Run%20to%20Player
  (if (!= (Variables|Default|GetHealth) 0.0)
    (AI|AIMoveTo self "0, 0, 0" (Variables|Default|GetAs%20BP%20Character) 5.0 false
      (:OnSuccess
        (CallFunction|RuntoPlayer)))))

(event EventBeginPlay
  (bind _asbp_hero (Utilities|Casting|CastToBP_Hero (Game|GetPlayerCharacter 0)))
  (Variables|Default|SetAs%20BP%20Character _asbp_hero)
  (CallFunction|RuntoPlayer))

(event Collision|EventActorBeginOverlap
  (params (OtherActor :type Actor%20Object%20Reference)))

(event EventTick
  (params (DeltaSeconds :type Float%20%28single-precision%29)))

(fn ConstructionScript)