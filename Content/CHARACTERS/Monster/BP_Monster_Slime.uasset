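; Slime monster Blueprint that spawns a smaller child slime as soon as it begins play.
; BeginPlay calls the parent, then passes an always-true branch to spawn one BP_Monster_Slime_Child at half this actor's scale.
; The multiply step is marked "BELUM" (Indonesian for "not yet"), and overlap, tick and construction add no logic of their own.
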(event EventBeginPlay
  (|CallParentFunction)
  ;[1 1 1] Multiply Slime BELUM
  (if true
    (Game|SpawnActorfromClass "/Game/CHARACTERS/Monster/BP_Monster_Slime_Child.BP_Monster_Slime_Child_C" (Math|Transform|MakeTransform "0, 0, 0" "0, 0, 0" (/ (Transformation|GetActorScale3D) "2.000000,2.000000,2.000000")) "Undefined" "MultiplyWithRoot" 0 0)))

(event Collision|EventActorBeginOverlap
  (params (OtherActor :type Actor%20Object%20Reference))
  (|CallParentFunction OtherActor) ; This node is disabled and will not be called.\nDrag off pins to build functionality.
)

(event EventTick
  (params (DeltaSeconds :type Float%20%28single-precision%29))
  (|CallParentFunction DeltaSeconds) ; This node is disabled and will not be called.\nDrag off pins to build functionality.
)

(fn ConstructionScript
  (|CallParentFunction))