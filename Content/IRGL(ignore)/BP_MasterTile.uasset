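; BP_MasterTile is a spawner actor that lays out a flat grid of BP_Tile actors when play begins.
; BeginPlay loops up to MaxActor, using the remainder and whole part of the index divided by MaxRow as X and Y steps, scaled by ActorSpacing and offset from its own location.
; The Spawn event and construction script are empty.
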(event Custom|Spawn)

(event EventBeginPlay
  (bind _actorspacing (Variables|Default|GetActorSpacing))
  (for _index (range 0 (Variables|Default|GetMax%20Actor))
    (Game|SpawnActorfromClass "/Game/IRGL(ignore)/BP_Tile.BP_Tile_C" (Math|Transform|MakeTransform (+ (Transformation|GetActorLocation) (Math|Vector|MakeVector (* (.Remainder (Math|Float|Division(WholeandRemainder) (Math|Conversions|ToFloat(Integer) _index) (Variables|Default|GetMax%20Row))) _actorspacing) (Math|Conversions|ToFloat(Integer) (* (Math|Conversions|ToFloat(Integer) (.ReturnValue (Math|Float|Division(WholeandRemainder) (Math|Conversions|ToFloat(Integer) _index) (Variables|Default|GetMax%20Row)))) _actorspacing)) 0.0)) "0, 0, 0" "1.000000,1.000000,1.000000") "Undefined" "MultiplyWithRoot" 0 0)))

(event Collision|EventActorBeginOverlap
  (params (OtherActor :type Actor%20Object%20Reference)))

(event EventTick
  (params (DeltaSeconds :type Float%20%28single-precision%29)))

(fn ConstructionScript)