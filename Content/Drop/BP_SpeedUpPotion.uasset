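; BP_SpeedUpPotion is a pickup that temporarily raises the hero's walk speed.
; When BP_Hero_ overlaps the box collision, it adds a fixed bonus to MaxWalkSpeed and hides the SpeedUp component.
; After a delay, it subtracts the same bonus and destroys itself.
; A First flag, cleared only after the hero cast succeeds, keeps the effect from triggering twice.
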(event OnComponentBeginOverlap(BoxCollision)
  (params (OverlappedComponent :type Primitive%20Component%20Object%20Reference) (OtherActor :type Actor%20Object%20Reference) (OtherComp :type Primitive%20Component%20Object%20Reference) (OtherBodyIndex :type Integer) (bFromSweep :type Boolean) (SweepResult :type Hit%20Result%20Structure%20%28by%20ref%29))
  ;[1 1 1] SpeedUp
  (if (Variables|Default|Getfirst?)
    (bind _asbp_hero_ (Utilities|Casting|CastToBP_Hero_ OtherActor))
    (Variables|Default|Setfirst? false)
    (Variables|/Script/Engine.CharacterMovementComponent|SetMaxWalkSpeed (Variables|/Script/Engine.Character|GetCharacterMovement _asbp_hero_) (+ (Variables|/Script/Engine.CharacterMovementComponent|GetMaxWalkSpeed (Variables|/Script/Engine.Character|GetCharacterMovement _asbp_hero_)) 1e+02))
    (Rendering|SetVisibility (Variables|Default|GetSpeedUp) false false)
    (Utilities|FlowControl|Delay 8.0)
    (Variables|/Script/Engine.CharacterMovementComponent|SetMaxWalkSpeed (Variables|/Script/Engine.Character|GetCharacterMovement _asbp_hero_) (- (Variables|/Script/Engine.CharacterMovementComponent|GetMaxWalkSpeed (Variables|/Script/Engine.Character|GetCharacterMovement _asbp_hero_)) 1e+02))
    (Actor|DestroyActor)))

(event EventBeginPlay)

(event Collision|EventActorBeginOverlap
  (params (OtherActor :type Actor%20Object%20Reference)))

(event EventTick
  (params (DeltaSeconds :type Float%20%28single-precision%29)))

(fn ConstructionScript)