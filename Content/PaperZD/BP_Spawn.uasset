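; BP_Spawn is a spawner actor that populates the level with BP_Chicken enemies when play begins.
; BeginPlay gathers all BP_SpawnPosition actors, then spawns chickens at random ones in a delayed loop until the enemy counter reaches its small limit.
; It also slows its tick interval, but Tick is empty and a chicken lookup node is left unconnected.
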(event EventBeginPlay
  (bind _outactors (Actor|GetAllActorsOfClass "/Game/PaperZD/BP_SpawnPosition.BP_SpawnPosition_C"))
  (Variables|Default|SetPosition _outactors)
  (Actor|Tick|SetActorTickInterval 5.0)
  (Game|SpawnActorfromClass "/Game/PaperZD/BP_Chicken.BP_Chicken_C" (Math|Transform|MakeTransform (Transformation|GetActorLocation (.OutItem (Utilities|Array|Random (Variables|Default|GetPosition)))) "0, 0, 0" "1.000000,1.000000,1.000000") "Undefined" "MultiplyWithRoot" 0 0 :!label _label)
  (bind _result (Math|Integer|IncrementInt (Variables|Default|GetCountEnemy))
    (:%20%20
      (Variables|Default|SetCountEnemy _result)
      (Utilities|FlowControl|Delay 1.0)
      (if (< (Variables|Default|GetCountEnemy) 3)
        (goto _label)))))

(event Collision|EventActorBeginOverlap
  (params (OtherActor :type Actor%20Object%20Reference)))

(event EventTick
  (params (DeltaSeconds :type Float%20%28single-precision%29)))

(fn ConstructionScript)