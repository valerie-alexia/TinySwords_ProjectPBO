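; BP_Character is a player-controlled sprite character that moves on the world X and Y axes and shoots fireballs.
; BeginPlay registers the Enhanced Input mapping, and the movement action drives movement input, mirroring the sprite by setting its X scale to the horizontal input value.
; The shoot action spawns BP_Projectile_FireBall at the ArrowShoot transform.
; A TimeJump timeline that would set the actor's Y location is present but never runs.
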(event Input|EnhancedActionEvents|EnhancedInputActionIA_shoot
  (params (ActionValue :type Float%20%28double-precision%29) (ElapsedSeconds :type Float%20%28double-precision%29) (TriggeredSeconds :type Float%20%28double-precision%29) (InputAction :type Input%20Action%20Object%20Reference :default "/Game/PaperZD/IA_shoot.IA_shoot"))
  (:Started
    (Game|SpawnActorfromClass "/Game/PaperZD/Skills/BP_Projectile_FireBall.BP_Projectile_FireBall_C" (Transformation|GetWorldTransform (Variables|Default|GetarrowShoot)) "Undefined" "MultiplyWithRoot" 0 0)))

(event Input|EnhancedActionEvents|EnhancedInputActionIA_Movement
  (params (ActionValue :type Vector%202D%20Structure) (ElapsedSeconds :type Float%20%28double-precision%29) (TriggeredSeconds :type Float%20%28double-precision%29) (InputAction :type Input%20Action%20Object%20Reference :default "/Game/PaperZD/IA_Movement.IA_Movement"))
  (:Triggered
    (Utilities|FlowControl|Sequence
      (:then_0
        (Pawn|Input|AddMovementInput "1.000000,0.000000,0.000000" (.x ActionValue) false)
        (if (!= (.x ActionValue) 0.0)
          (Transformation|SetWorldScale3D (Variables|Default|GetSprite) (Math|Vector|MakeVector (.x ActionValue) 1.0 1.0))))
      (:then_1
        (Pawn|Input|AddMovementInput "0.000000,-1.000000,0.000000" (.y ActionValue) false)))))

(event EventBeginPlay
  (bind _asplayer_controller (Utilities|Casting|CastToPlayerController (Game|GetPlayerController 0)))
  (Utilities|IsValid (PlayerController|LocalPlayerSubsystems|GetEnhancedInputLocalPlayerSubsystem _asplayer_controller)
    (:Is%20Valid
      (Input|AddMappingContext (PlayerController|LocalPlayerSubsystems|GetEnhancedInputLocalPlayerSubsystem _asplayer_controller) "/Game/PaperZD/IMC_MovementMapping.IMC_MovementMapping" 0 "(bIgnoreAllPressedKeysUntilRelease=True,bForceImmediately=False,bNotifyUserSettings=False)"))))

(event Collision|EventActorBeginOverlap
  (params (OtherActor :type Actor%20Object%20Reference)))

(event EventTick
  (params (DeltaSeconds :type Float%20%28single-precision%29)))

(fn ConstructionScript)